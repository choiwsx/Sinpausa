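; Monster that walks along its mesh's right vector at its status speed and destroys itself once HP runs out.
; AnyDamage casts the damage type to Fire, Thunder or Ice and subtracts its final damage from HP.
; Fire adds a looping-timer burn DOT, while Thunder and Ice scale speed until their counters pass MaxCount.
; All effects share one Count, CurrentDamage and timer handle, and end by pausing the timer.
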(event Custom|Freeze%20Count
  ;[1 1 1] Ice Damage & Slow
  (bind _result (Math|Integer|IncrementInt (Variables|Default|GetCount))
    (:%20%20
      (if (> _result (Variables|Default|GetMaxCount))
        (Variables|Default|SetCount 0)
        (Utilities|Time|PauseTimerbyHandle (Variables|Default|GetTimerhandle))
        (Variables|/Game/BluePrints/Monster/BP_MonsterStatus.BP_MonsterStatus_C|SetSpeed (Variables|Default|GetBP_MonsterStatus) (stale Game|Damage|EventAnyDamage _output_get_2))
        (Variables|Default|SetCurrentDamage 0.0)))))

(event Custom|Pause%20Count
  ;[1 1 1] Thunder Damage & Pause
  (bind _result (Math|Integer|IncrementInt (Variables|Default|GetCount))
    (:%20%20
      (if (> _result (Variables|Default|GetMaxCount))
        (Variables|Default|SetCount 0)
        (Utilities|Time|PauseTimerbyHandle (Variables|Default|GetTimerhandle))
        (Variables|/Game/BluePrints/Monster/BP_MonsterStatus.BP_MonsterStatus_C|SetSpeed (Variables|Default|GetBP_MonsterStatus) (stale Game|Damage|EventAnyDamage _output_get))
        (Variables|Default|SetCurrentDamage 0.0)))))

(event Custom|ProcessDamage
  ;[1 1 1] Fire Damage & DOT
  (Variables|Default|SetCurrentDamage (Variables|/Game/BluePrints/AllTower/MagicTower/DamageType/BP_DamageBase.BP_DamageBase_C|GetDOT (stale Game|Damage|EventAnyDamage _asbp_fire_type)))
  (CallFunction|Burn) ; 화상
  (bind _result (Math|Integer|IncrementInt (Variables|Default|GetCount))
    (:%20%20
      (if (> _result 3)
        (Variables|Default|SetCount 0)
        (Utilities|Time|PauseTimerbyHandle (Variables|Default|GetTimerhandle))
        (Variables|Default|SetCurrentDamage 0.0)))))

(event Game|Damage|EventAnyDamage
  (params (Damage :type Float%20%28single-precision%29) (DamageType :type Damage%20Type%20Object%20Reference) (InstigatedBy :type Controller%20Object%20Reference) (DamageCauser :type Actor%20Object%20Reference))
  ;[1 1 1] Fire Damage & DOT
  (bind _asbp_fire_type (Utilities|Casting|CastToBP_FireType DamageType)
    (:then
      (Variables|Default|SetCurrentDamage (Variables|/Game/BluePrints/AllTower/MagicTower/DamageType/BP_DamageBase.BP_DamageBase_C|GetFinalDamage _asbp_fire_type))
      (CallFunction|Damage) ; 불
      (CallFunction|ProcessDamage)
      (bind _returnvalue (Utilities|Time|SetTimerbyEvent (delegate Custom|ProcessDamage) 1.0 true))
      (Variables|Default|SetTimerhandle _returnvalue))
    (:CastFailed
      ;[1 1 1] Thunder Damage & Pause
      (bind _asbp_thunder_type (Utilities|Casting|CastToBP_ThunderType DamageType)
        (:then
          (Variables|Default|SetCurrentDamage (Variables|/Game/BluePrints/AllTower/MagicTower/DamageType/BP_DamageBase.BP_DamageBase_C|GetFinalDamage _asbp_thunder_type))
          (bind _output_get (Variables|Default|SetNormalSpeed (Variables|/Game/BluePrints/Monster/BP_MonsterStatus.BP_MonsterStatus_C|GetSpeed (Variables|Default|GetBP_MonsterStatus))))
          (CallFunction|Damage) ; 번개
          (CallFunction|SpeedChange (Variables|/Game/BluePrints/AllTower/MagicTower/DamageType/BP_DamageBase.BP_DamageBase_C|GetFinalSpeed _asbp_thunder_type))
          (bind _returnvalue_2 (Utilities|Time|SetTimerbyEvent (delegate Custom|Pause%20Count) 1.0 true))
          (Variables|Default|SetTimerhandle _returnvalue_2))
        (:CastFailed
          ;[1 1 1] Ice Damage & Slow
          (bind _asbp_ice_type (Utilities|Casting|CastToBP_IceType DamageType))
          (Variables|Default|SetCurrentDamage (Variables|/Game/BluePrints/AllTower/MagicTower/DamageType/BP_DamageBase.BP_DamageBase_C|GetFinalDamage _asbp_ice_type))
          (bind _output_get_2 (Variables|Default|SetNormalSpeed (Variables|/Game/BluePrints/Monster/BP_MonsterStatus.BP_MonsterStatus_C|GetSpeed (Variables|Default|GetBP_MonsterStatus))))
          (CallFunction|Damage) ; 얼음
          (CallFunction|SpeedChange (Variables|/Game/BluePrints/AllTower/MagicTower/DamageType/BP_DamageBase.BP_DamageBase_C|GetFinalSpeed _asbp_ice_type))
          (bind _returnvalue_3 (Utilities|Time|SetTimerbyEvent (delegate Custom|Freeze%20Count) 1.0 true))
          (Variables|Default|SetTimerhandle _returnvalue_3))))))

(event EventTick
  (params (DeltaSeconds :type Float%20%28single-precision%29))
  ;[1 1 1] 이동 & 죽음판정
  (Pawn|Input|AddMovementInput (Math|Vector|GetRightVector (Variables|Character|GetMesh)) (Variables|/Game/BluePrints/Monster/BP_MonsterStatus.BP_MonsterStatus_C|GetSpeed (Variables|Default|GetBP_MonsterStatus)) false)
  (CallFunction|Dead))

(fn ConstructionScript)

(fn Dead
  (if (<= (Variables|/Game/BluePrints/Monster/BP_MonsterStatus.BP_MonsterStatus_C|GetHP (Variables|Default|GetBP_MonsterStatus)) 0.0)
    (Actor|DestroyActor)
    (Development|PrintString "Dead"))
  (return))

(fn Damage
  (bind _bp_monsterstatus (Variables|Default|GetBP_MonsterStatus))
  (bind _output_get (Variables|/Game/BluePrints/Monster/BP_MonsterStatus.BP_MonsterStatus_C|SetHP _bp_monsterstatus (- (Variables|/Game/BluePrints/Monster/BP_MonsterStatus.BP_MonsterStatus_C|GetHP _bp_monsterstatus) (Variables|Default|GetCurrentDamage))))
  (Development|PrintString (Utilities|String|ToString(Float) _output_get))
  (return))

(fn SpeedChange
  (params (SpeedType :type Float%20%28single-precision%29))
  (bind _bp_monsterstatus (Variables|Default|GetBP_MonsterStatus))
  (Variables|/Game/BluePrints/Monster/BP_MonsterStatus.BP_MonsterStatus_C|SetSpeed _bp_monsterstatus (* SpeedType (Variables|/Game/BluePrints/Monster/BP_MonsterStatus.BP_MonsterStatus_C|GetSpeed _bp_monsterstatus)))
  (return))

(fn CountTime
  (bind _result (Math|Integer|IncrementInt (Variables|Default|GetCount))
    (:%20%20
      (if (> _result 3)
        (Variables|Default|SetCount 0))
      (return))))

(fn Burn
  (bind _bp_monsterstatus (Variables|Default|GetBP_MonsterStatus))
  (Variables|/Game/BluePrints/Monster/BP_MonsterStatus.BP_MonsterStatus_C|SetHP _bp_monsterstatus (- (Variables|/Game/BluePrints/Monster/BP_MonsterStatus.BP_MonsterStatus_C|GetHP _bp_monsterstatus) (Variables|Default|GetCurrentDamage)))
  (return))