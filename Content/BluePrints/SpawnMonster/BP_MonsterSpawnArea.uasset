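; BP_MonsterSpawnArea is a trigger area that turns monster dolls into monsters when they enter its box.
; On overlap, it casts the other actor to BP_MonsterDollBase and looks up the doll's MonsterNum as a row name in DT_Monster.
; If the row exists, it spawns that row's MonsterClass at the sweep impact point with a fixed rotation, then destroys the doll.
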(event OnComponentBeginOverlap(Box)
  (params (OverlappedComponent :type Primitive%20Component%20Object%20Reference) (OtherActor :type Actor%20Object%20Reference) (OtherComp :type Primitive%20Component%20Object%20Reference) (OtherBodyIndex :type Integer) (bFromSweep :type Boolean) (SweepResult :type Hit%20Result%20Structure%20%28by%20ref%29))
  (bind _asbp_monster_doll_base (Utilities|Casting|CastToBP_MonsterDollBase OtherActor))
  (Variables|Default|SetMonsterDoll _asbp_monster_doll_base)
  (bind _returnvalue (Utilities|GetDataTableRow "/Game/AI/Monster/Struct/DT_Monster.DT_Monster" (Utilities|String|StringToName (Utilities|String|ToString(Integer) (Variables|/Game/BluePrints/SpawnMonster/BP_MonsterDollBase.BP_MonsterDollBase_C|GetMonsterNum _asbp_monster_doll_base))))
    (:then
      (Game|SpawnActorfromClass (.MonsterClass (Utilities|Struct|BreakST_Monster _returnvalue)) (Math|Transform|MakeTransform (.ImpactPoint (Collision|BreakHitResult SweepResult)) "0,180.000000, 0") "Undefined" 0 0 0)
      (Actor|DestroyActor (Variables|Default|GetMonsterDoll)))))

(event EventBeginPlay)

(fn ConstructionScript)