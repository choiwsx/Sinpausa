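; BP_BowHeroTower is a barracks-type hero tower that spawns a BP_BasicBow actor when play begins.
; BeginPlay runs the parent logic, then spawns the bow slightly offset from and above the tower, adjusting for collisions but always spawning.
; The construction script and overlap event only call the parent, and Tick is disabled.
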(event EventBeginPlay
  (|CallParentFunction)
  (Game|SpawnActorfromClass "/Game/AI/Hero/BP_BasicBow.BP_BasicBow_C" (Math|Transform|MakeTransform (+ (Transformation|GetActorLocation) "0,15.000000,20.000000")) "AdjustIfPossibleButAlwaysSpawn" 0 0 0))

(event Collision|EventActorBeginOverlap
  (params (OtherActor :type Actor%20Object%20Reference))
  (|CallParentFunction OtherActor))

(event EventTick
  (params (DeltaSeconds :type Float%20%28single-precision%29))
  (|CallParentFunction DeltaSeconds) ; 지금 이 노드는 비활성 상태입니다. \n핀을 끌어서 다른 노드를 연결하면 활성화됩니다.
)

(fn ConstructionScript
  (|CallParentFunction))