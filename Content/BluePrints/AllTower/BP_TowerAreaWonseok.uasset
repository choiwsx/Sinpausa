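; BP_TowerAreaWonseok is a VR tower build spot that opens a build menu when a motion controller touches its static mesh.
; The overlap is handled only without authority and only for the local player's controller that is not already building.
; If its Widget_Build has no owning tower, it reveals and initializes the widget with this area and controller.
; It then activates the controller's widget interaction and flags it as building.
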(event OnComponentBeginOverlap(StaticMesh)
  (params (OverlappedComponent :type Primitive%20Component%20Object%20Reference) (OtherActor :type Actor%20Object%20Reference) (OtherComp :type Primitive%20Component%20Object%20Reference) (OtherBodyIndex :type Integer) (bFromSweep :type Boolean) (SweepResult :type Hit%20Result%20Structure%20%28by%20ref%29))
  (Networking|SwitchHasAuthority
    (:Remote
      (CallFunction|11 OtherActor))))

(event Custom|11
  (params (NewParam :type Actor%20Object%20Reference))
  (bind _widget (Variables|Default|GetWidget))
  (bind _asbp_motion_controller (Utilities|Casting|CastToBP_MotionController NewParam))
  (Variables|Default|SetMotionController _asbp_motion_controller)
  (bind _asmotion_controller_pawn (Utilities|Casting|CastToMotionControllerPawn (Components|GetOwner _asbp_motion_controller)))
  (if (== (Pawn|GetController _asmotion_controller_pawn) (Game|GetPlayerController 0))
    (Utilities|IsValid (Variables|Default|GetMotionController)
      (:Is%20Valid
        (if (not (Variables|/Game/VirtualRealityBP/Blueprints/BP_MotionController.BP_MotionController_C|GetIsBuilding? _asbp_motion_controller))
          (bind _aswidget_build (Utilities|Casting|CastToWidget_Build (UserInterface|GetUserWidgetObject _widget)))
          (Utilities|IsValid _aswidget_build
            (:Is%20Valid
              (Variables|Default|SetBuildWidget _aswidget_build)
              (Utilities|IsValid (Variables|/Game/AI/Build/Widget/Widget_Build.Widget_Build_C|GetOwnTower (Variables|Default|GetBuildWidget))
                (:Is%20Not%20Valid
                  (Development|SetHiddeninGame _widget false false)
                  (Variables|/Game/AI/Build/Widget/Widget_Build.Widget_Build_C|SetOwnTower (Variables|Default|GetBuildWidget) self)
                  (Variables|/Game/AI/Build/Widget/Widget_Build.Widget_Build_C|SetMotionController (Variables|Default|GetBuildWidget) (Variables|Default|GetMotionController))
                  (Default|Initial (Variables|Default|GetBuildWidget))
                  (Components|Activation|Activate (Variables|/Game/VirtualRealityBP/Blueprints/BP_MotionController.BP_MotionController_C|GetWidgetInteraction (Variables|Default|GetMotionController)) false)
                  (Variables|/Game/VirtualRealityBP/Blueprints/BP_MotionController.BP_MotionController_C|SetIsBuilding? (Variables|Default|GetMotionController) true))))))))))

(event EventBeginPlay)

(event Collision|EventActorBeginOverlap
  (params (OtherActor :type Actor%20Object%20Reference)))

(fn ConstructionScript)