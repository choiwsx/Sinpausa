(event OnComponentBeginOverlap(Sphere)
  (params (OverlappedComponent :type Primitive%20Component%20Object%20Reference) (OtherActor :type Actor%20Object%20Reference) (OtherComp :type Primitive%20Component%20Object%20Reference) (OtherBodyIndex :type Integer) (bFromSweep :type Boolean) (SweepResult :type Hit%20Result%20Structure%20%28by%20ref%29))
  (Utilities|Casting|CastToBP_MotionController OtherActor)
  (CallFunction|CheckMagic))

(event Custom|FireSpawn
  (Utilities|Casting|CastToPC_Controller (Game|GetPlayerController 0))
  (Game|SpawnActorfromClass "/Game/BluePrints/AllTower/MagicTower/BP_Fire.BP_Fire_C" (Math|Transform|MakeTransform (+ (Transformation|GetActorLocation) "0, 0,35.000000") (Transformation|GetActorRotation) "0.020000,0.020000,0.020000") "AlwaysSpawn" self self "2" 0)
  (Variables|Default|SetMake true))

(event Custom|CheckMagic
  (if (not (Variables|Default|GetMake))
    (CallFunction|FireSpawn)))

(event EventBeginPlay
  (Variables|Default|SetMake false))

(fn ConstructionScript
  (|CallParentFunction))