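; Level 1 fire magic tower that spawns a small BP_Fire actor just above itself, passing itself as its Tower.
; Tick spawns the fire after a one-second Delay and sets Make to block further spawns until CustomEvent clears it.
; TowerMesh overlap events toggle an Overlap flag, which this graph never reads.
; The construction script only calls the parent.
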(event OnComponentBeginOverlap(TowerMesh)
  (params (OverlappedComponent :type Primitive%20Component%20Object%20Reference) (OtherActor :type Actor%20Object%20Reference) (OtherComp :type Primitive%20Component%20Object%20Reference) (OtherBodyIndex :type Integer) (bFromSweep :type Boolean) (SweepResult :type Hit%20Result%20Structure%20%28by%20ref%29))
  (Variables|Default|SetOverlap true))

(event OnComponentEndOverlap(TowerMesh)
  (params (OverlappedComponent :type Primitive%20Component%20Object%20Reference) (OtherActor :type Actor%20Object%20Reference) (OtherComp :type Primitive%20Component%20Object%20Reference) (OtherBodyIndex :type Integer))
  (Variables|Default|SetOverlap false))

(event Custom|CustomEvent
  (Variables|Default|SetMake false))

(event EventTick
  (params (DeltaSeconds :type Float%20%28single-precision%29))
  (if (not (Variables|Default|GetMake))
    (Utilities|FlowControl|Delay 1.0)
    (Game|SpawnActorfromClass "/Game/BluePrints/AllTower/MagicTower/BP_Fire.BP_Fire_C" (Math|Transform|MakeTransform (+ (Transformation|GetActorLocation) "0, 0,20.000000") "0, 0, 0" "0.030000,0.030000,0.030000") "Undefined" 0 self "2" 0)
    (Variables|Default|SetMake true)))

(fn ConstructionScript
  (|CallParentFunction))