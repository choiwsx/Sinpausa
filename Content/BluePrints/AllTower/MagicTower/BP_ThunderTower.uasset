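; BP_ThunderTower is a magic tower that spawns a single BP_Thunder actor just above itself shortly after play begins.
; Tick runs a one-second Delay behind the Make flag, then spawns the tiny-scaled thunder with a tower self-reference and TowerStruct value, and sets Make.
; TowerMesh begin and end overlap events toggle an Overlap flag, which this graph does not read.
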(event OnComponentBeginOverlap(TowerMesh)
  (params (OverlappedComponent :type Primitive%20Component%20Object%20Reference) (OtherActor :type Actor%20Object%20Reference) (OtherComp :type Primitive%20Component%20Object%20Reference) (OtherBodyIndex :type Integer) (bFromSweep :type Boolean) (SweepResult :type Hit%20Result%20Structure%20%28by%20ref%29))
  (Variables|Default|SetOverlap true))

(event OnComponentEndOverlap(TowerMesh)
  (params (OverlappedComponent :type Primitive%20Component%20Object%20Reference) (OtherActor :type Actor%20Object%20Reference) (OtherComp :type Primitive%20Component%20Object%20Reference) (OtherBodyIndex :type Integer))
  (Variables|Default|SetOverlap false))

(event Collision|EventActorBeginOverlap
  (params (OtherActor :type Actor%20Object%20Reference))
  (|CallParentFunction OtherActor) ; 지금 이 노드는 비활성 상태입니다. \n핀을 끌어서 다른 노드를 연결하면 활성화됩니다.
)

(event EventTick
  (params (DeltaSeconds :type Float%20%28single-precision%29))
  (if (not (Variables|Default|GetMake))
    (Utilities|FlowControl|Delay 1.0)
    (Game|SpawnActorfromClass "/Game/BluePrints/AllTower/MagicTower/BP_Thunder.BP_Thunder_C" (Math|Transform|MakeTransform (+ (Transformation|GetActorLocation) "0, 0,20.000000") "0, 0, 0" "0.002000,0.002000,0.002000") "Undefined" 0 self "4" 0)
    (Variables|Default|SetMake true)))

(event EventBeginPlay
  (Variables|Default|SetMake false))

(fn ConstructionScript
  (|CallParentFunction))