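; Monster character, apparently a test variant under ArrowTest, that walks along a spline with a random X/Y offset while in PEACE.
; Events cover nearest-hero aggro, countering, capsule-trace melee with knockback, and timer callbacks for fire, ice and lightning effects.
; SetState, AnyDamage and pawn sensing are empty.
; State speeds and montages, hit reactions, status-timer setup and death with gold drop exist only as disconnected nodes, so never run.
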(event OnSeePawn(PawnSensing)
  (params (Pawn :type Pawn%20Object%20Reference))
  ;[1 1 1] OnSeePawn 이벤트
)

(event Custom|SetState
  (params (NewState :type BPE_MonsterState%20Enum :default "NewEnumerator0"))
  ;[1 1 1] SetState 이벤트
)

(event Custom|Combo2_monster
  (CallFunction|SetState "NewEnumerator5"))

(event Custom|AggroCheck
  (Variables|Default|SetDistanceToHero 3e+01)
  (Variables|Default|SetTargetHero 0)
  (bind _outactors (Actor|GetAllActorsOfClass "/Game/AI/Hero/BP_HERO_BASE.BP_HERO_BASE_C"))
  (for _array_element _outactors
    (if (< (Math|Vector|VectorLength (- (Transformation|GetActorLocation) (Transformation|GetActorLocation _array_element))) (Variables|Default|GetDistanceToHero))
      (Variables|Default|SetDistanceToHero (Math|Vector|VectorLength (- (Transformation|GetActorLocation) (Transformation|GetActorLocation _array_element))))
      (Variables|Default|SetTargetHero _array_element)))
  (if (<= (Variables|Default|GetDistanceToHero) 8e+02)
    (Utilities|IsValid (Variables|Default|GetTargetHero)
      (:Is%20Valid
        (if (< (Utilities|Array|Length (Variables|/Game/AI/Hero/BP_HERO_BASE.BP_HERO_BASE_C|GetBattleMonsterArray (Variables|Default|GetTargetHero))) (Variables|Default|GetMaxBattelMonsterCount))
          (Variables|Actor|SetInstigator (Variables|Default|GetTargetHero))
          (CallFunction|SetState "NewEnumerator1"))))))

(event Custom|BasicAttack
  (params (Damage :type Float%20%28single-precision%29))
  (bind _returnvalue (Transformation|GetActorLocation))
  ;[1 1 1] 몬스터 베이직 어택
  (bind _outactors (Actor|GetAllActorsOfClass "/Game/AI/Monster/BP_Monster_BASIC.BP_Monster_BASIC_C"))
  (bind _outhit (Class|KismetSystemLibrary|CapsuleTraceSingleforObjects _returnvalue (+ _returnvalue (* (Transformation|GetActorForwardVector) 6.0)) 4.0 3.0 (Utilities|Array|MakeArray "ObjectTypeQuery3") false _outactors "ForDuration" true "(R=0.000000,G=0.207014,B=1.000000,A=1.000000)" "(R=1.000000,G=0.000000,B=0.951921,A=1.000000)"))
  (bind _asbp_hero_base (Utilities|Casting|CastToBP_HERO_BASE (.HitActor (Collision|BreakHitResult _outhit))))
  (Utilities|IsValid _asbp_hero_base
    (:Is%20Valid
      (Physics|AddImpulse (Variables|/Script/Engine.Character|GetCharacterMovement _asbp_hero_base) (* (Transformation|GetActorForwardVector _asbp_hero_base) -1e+01) false)
      (Game|Damage|ApplyDamage _asbp_hero_base Damage 0 self))))

(event Custom|Combo2_Impulse
  (Physics|AddImpulse (Variables|Character|GetCharacterMovement) (* (Transformation|GetActorForwardVector) -5.0) true))

(event Custom|Counter
  (params (Hero :type BP%20HERO%20BASE%20Object%20Reference))
  (if (< (Utilities|Array|Length (Variables|/Game/AI/Hero/BP_HERO_BASE.BP_HERO_BASE_C|GetBattleMonsterArray Hero)) (Variables|Default|GetMaxBattelMonsterCount))
    (Variables|Actor|SetInstigator Hero)
    (CallFunction|SetState "NewEnumerator1")
    (bind _asbp_hero_base (Utilities|Casting|CastToBP_HERO_BASE Hero))
    (Math|Integer|IncrementInt (Variables|/Game/AI/Hero/BP_HERO_BASE.BP_HERO_BASE_C|GetBattleMonsterCount _asbp_hero_base))))

(event Custom|DOT
  ;[1 1 1] 불 데미지
  (Utilities|IsValid 0
    (:Is%20Valid
      (Variables|Default|SetCurrentHP (- (Variables|Default|GetCurrentHP) 1.0))
      (bind _result (Math|Integer|IncrementInt (Variables|Default|GetCount))
        (:%20%20
          (if (> _result 2) ; 시간이 다 되면 True
            (Utilities|Time|PauseTimerbyHandle (Variables|Default|GetTiemHandle))))))))

(event Custom|Shock
  ;[1 1 1] 번개 데미지
  (bind _result (Math|Integer|IncrementInt (Variables|Default|GetCount))
    (:%20%20
      (if (> _result (Variables|Default|Getduration)) ; 시간이 다 되면 True
        (Utilities|Time|PauseTimerbyHandle (Variables|Default|GetTiemHandle))
        (Variables|Default|SetCurrentSpeed 5.0)
        (Variables|Default|SetCount 0)))))

(event Custom|Slow
  ;[1 1 1] 얼음 데미지
  (bind _result (Math|Integer|IncrementInt (Variables|Default|GetCount))
    (:%20%20
      (if (> _result (Variables|Default|Getduration)) ; 시간이 다 되면 True
        (Utilities|Time|PauseTimerbyHandle (Variables|Default|GetTiemHandle))
        (Variables|Default|SetCurrentSpeed 5.0)
        (Variables|Default|SetCount 0)))))

(event EventBeginPlay
  ;[1 1 1] Begin Play 이벤트
  (Variables|Default|SetCurrentHP (Variables|Default|GetMaxHP))
  (bind _aswidget_monster_hp (Utilities|Casting|CastToWidget_MonsterHP (UserInterface|GetUserWidgetObject (Variables|Default|GetWidget))))
  (Progress|SetPercent (Variables|/Game/AI/Monster/Widget/Widget_MonsterHP.Widget_MonsterHP_C|GetHP _aswidget_monster_hp) (/ (Variables|Default|GetCurrentHP) (Variables|Default|GetMaxHP)))
  (CallFunction|SetState "NewEnumerator0")
  (Variables|Default|SetOffset (Math|Random|RandomFloatinRange -7.0 7.0)))

(event Collision|EventActorBeginOverlap
  (params (OtherActor :type Actor%20Object%20Reference))
  (|CallParentFunction OtherActor) ; 지금 이 노드는 비활성 상태입니다. \n핀을 끌어서 다른 노드를 연결하면 활성화됩니다.
)

(event EventTick
  (params (DeltaSeconds :type Float%20%28single-precision%29))
  (bind _spline_ref (Variables|Default|GetSpline_Ref))
  (bind _spline (Variables|/Game/AI/Monster/Spline_Base.Spline_Base_C|GetSpline _spline_ref))
  ;[1 1 1] Tick 이벤트
  (Utilities|FlowControl|Sequence
    (:then_1
      (if (Utilities|Enum|Equal(Enum) (Variables|Default|GetCurrentState) "NewEnumerator0")
        (Utilities|IsValid (Variables|Default|GetSpline_Ref)
          (:Is%20Valid
            (Variables|Default|SetDistanceAlongSpline (+ (* (* (Variables|Default|GetCurrentSpeed) (Variables|Default|GetAxisValue)) (Utilities|Time|GetWorldDeltaSeconds)) (Variables|Default|GetDistanceAlongSpline)))
            (Transformation|SetActorLocation (Math|Vector|MakeVector (+ (Variables|Default|GetOffset) (.x (Spline|GetLocationatDistanceAlongSpline _spline (Variables|Default|GetDistanceAlongSpline) "World"))) (+ (.y (Spline|GetLocationatDistanceAlongSpline _spline (Variables|Default|GetDistanceAlongSpline) "World")) (Variables|Default|GetOffset)) (.z (Transformation|GetActorLocation))) false false)
            (Transformation|SetActorRelativeRotation (Spline|GetRotationatDistanceAlongSpline _spline (Variables|Default|GetDistanceAlongSpline) "World"))
            (Variables|Default|SetB_PEACE_WALK true)))
        (else
          (Variables|Default|SetB_PEACE_WALK false))))))

(event Game|Damage|EventAnyDamage
  (params (Damage :type Float%20%28single-precision%29) (DamageType :type Damage%20Type%20Object%20Reference) (InstigatedBy :type Controller%20Object%20Reference) (DamageCauser :type Actor%20Object%20Reference))
  ;[1 1 1] AnyDamage 이벤트
)

(fn ConstructionScript
  (|CallParentFunction))