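; BP_TowerBow is an unfinished bow tower Blueprint from an arrow test, with target and firing logic only partly wired.
; Any overlap on its Sphere stores all BP_Monster_BASIC actors in the level in NewVar0, but no live logic reads that array.
; Tick forces the actor's rotation to zero every frame, so it does not aim.
; The muzzle effect and Arrow spawn at the left-hand bow socket are disconnected and never run.
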(event OnComponentBeginOverlap(Sphere)
  (params (OverlappedComponent :type Primitive%20Component%20Object%20Reference) (OtherActor :type Actor%20Object%20Reference) (OtherComp :type Primitive%20Component%20Object%20Reference) (OtherBodyIndex :type Integer) (bFromSweep :type Boolean) (SweepResult :type Hit%20Result%20Structure%20%28by%20ref%29))
  (bind _outactors (Actor|GetAllActorsOfClass "/Game/AI/Monster/BP_Monster_BASIC.BP_Monster_BASIC_C"))
  (Variables|Default|SetNewVar_0 _outactors))

(event EventBeginPlay)

(event Collision|EventActorBeginOverlap
  (params (OtherActor :type Actor%20Object%20Reference)))

(event EventTick
  (params (DeltaSeconds :type Float%20%28single-precision%29))
  (Transformation|SetActorRotation "0, 0, 0"))

(fn ConstructionScript)