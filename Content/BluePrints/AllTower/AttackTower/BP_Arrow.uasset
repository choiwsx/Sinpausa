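; BP_Arrow is a homing projectile, filed under attack towers, that damages monsters.
; On BeginPlay it scans all BP_Monster_BASIC actors for the nearest within Distance, homes ProjectileMovement onto it and sets a short lifespan.
; It destroys itself if no target is found or the target becomes invalid.
; Sphere overlap with any monster spawns an impact particle, applies Damage with the owner as causer and destroys the arrow.
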(event OnComponentBeginOverlap(Sphere)
  (params (OverlappedComponent :type Primitive%20Component%20Object%20Reference) (OtherActor :type Actor%20Object%20Reference) (OtherComp :type Primitive%20Component%20Object%20Reference) (OtherBodyIndex :type Integer) (bFromSweep :type Boolean) (SweepResult :type Hit%20Result%20Structure%20%28by%20ref%29))
  (bind (_bblockinghit _binitialoverlap _time _distance _location _impactpoint _normal _impactnormal) (Collision|BreakHitResult SweepResult))
  (bind _asbp_monster_basic (Utilities|Casting|CastToBP_Monster_BASIC OtherActor))
  (Utilities|IsValid _asbp_monster_basic
    (:Is%20Valid
      (Effects|SpawnEmitteratLocation "/Game/GabrielAguiarProd/ToonProjectilesVol1/Particles/Hits/P_Hit_Bullet01Blue.P_Hit_Bullet01Blue" _impactpoint (Math|Conversions|RotationFromXVector _impactnormal) "0.050000,0.050000,0.050000")
      (Game|Damage|ApplyDamage _asbp_monster_basic (Variables|Default|GetDamage) 0 (Components|GetOwner))
      (Actor|DestroyActor))))

(event EventBeginPlay
  (bind _outactors (Actor|GetAllActorsOfClass "/Game/AI/Monster/BP_Monster_BASIC.BP_Monster_BASIC_C"))
  (for _array_element _outactors
    (if (< (Math|Vector|VectorLength (- (Transformation|GetActorLocation _array_element) (Transformation|GetActorLocation))) (Variables|Default|GetDistance))
      (Variables|Default|SetDistance (Math|Vector|VectorLength (- (Transformation|GetActorLocation _array_element) (Transformation|GetActorLocation))))
      (Variables|Default|SetTargetMonster _array_element)))
  (Utilities|IsValid (Variables|Default|GetTargetMonster)
    (:Is%20Valid
      (Variables|/Script/Engine.ProjectileMovementComponent|SetHomingTargetComponent (Variables|Default|GetProjectileMovement) (Variables|/Script/Engine.Actor|GetRootComponent (Variables|Default|GetTargetMonster)))
      (Actor|SetLifeSpan 3.0))
    (:Is%20Not%20Valid
      (Actor|DestroyActor))))

(event EventTick
  (params (DeltaSeconds :type Float%20%28single-precision%29))
  (Utilities|IsValid (Variables|Default|GetTargetMonster)
    (:Is%20Not%20Valid
      (Actor|DestroyActor))))

(fn ConstructionScript)