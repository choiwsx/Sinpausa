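; Level 2 cannon attack tower Blueprint that spawns its cannon when play begins.
; After the parent BeginPlay, it looks up its fixed row in BP_HRDataTable for the attack delay.
; On success, it spawns a BP_Cannon slightly above its location, passing the row name, itself as owning tower and that delay as attack speed.
; Overlap, Tick and construction add no logic of their own.
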(event EventBeginPlay
  (|CallParentFunction)
  (bind _returnvalue (Utilities|GetDataTableRow "/Game/HR/BP_HRDataTable.BP_HRDataTable" "3")
    (:then
      (Game|SpawnActorfromClass "/Game/BluePrints/AllTower/AttackTower/BP_Cannon.BP_Cannon_C" (Math|Transform|MakeTransform (+ (Transformation|GetActorLocation) "0.350000, 0,13.000000")) "Undefined" 0 "3" self (.TowerAttackDelay (Utilities|Struct|BreakBP_HRStruct _returnvalue)) 0))))

(event Collision|EventActorBeginOverlap
  (params (OtherActor :type Actor%20Object%20Reference))
  (|CallParentFunction OtherActor) ; 지금 이 노드는 비활성 상태입니다. \n핀을 끌어서 다른 노드를 연결하면 활성화됩니다.
)

(event EventTick
  (params (DeltaSeconds :type Float%20%28single-precision%29))
  (|CallParentFunction DeltaSeconds) ; 지금 이 노드는 비활성 상태입니다. \n핀을 끌어서 다른 노드를 연결하면 활성화됩니다.
)

(fn ConstructionScript
  (|CallParentFunction))