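; BP_Projectile is an attack tower projectile that homes in on the nearest BP_Monster_BASIC and explodes on hit.
; On BeginPlay it scans all monsters, picks the closest as the homing target and sets a short lifespan.
; It destroys itself when no valid target exists, checked again every Tick.
; Hit applies small-radius, full radial damage with a scaled-down explosion, then destroys the actor; the sphere overlap handler is empty.
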(event OnComponentBeginOverlap(Sphere)
  (params (OverlappedComponent :type Primitive%20Component%20Object%20Reference) (OtherActor :type Actor%20Object%20Reference) (OtherComp :type Primitive%20Component%20Object%20Reference) (OtherBodyIndex :type Integer) (bFromSweep :type Boolean) (SweepResult :type Hit%20Result%20Structure%20%28by%20ref%29)))

(event EventBeginPlay
  (bind _outactors (Actor|GetAllActorsOfClass "/Game/AI/Monster/BP_Monster_BASIC.BP_Monster_BASIC_C"))
  (for _array_element _outactors
    (if (< (Math|Vector|VectorLength (- (Transformation|GetActorLocation _array_element) (Transformation|GetActorLocation))) (Variables|Default|GetDistance))
      (Variables|Default|SetDistance (Math|Vector|VectorLength (- (Transformation|GetActorLocation _array_element) (Transformation|GetActorLocation))))
      (Variables|Default|SetTargetMonster _array_element)))
  (Utilities|IsValid (Variables|Default|GetTargetMonster)
    (:Is%20Valid
      (Variables|/Script/Engine.ProjectileMovementComponent|SetHomingTargetComponent (Variables|Default|GetProjectileMovement) (Variables|/Script/Engine.Actor|GetRootComponent (Variables|Default|GetTargetMonster)))
      (Actor|SetLifeSpan 3.0))
    (:Is%20Not%20Valid
      (Actor|DestroyActor))))

(event EventTick
  (params (DeltaSeconds :type Float%20%28single-precision%29))
  (Utilities|IsValid (Variables|Default|GetTargetMonster)
    (:Is%20Not%20Valid
      (Actor|DestroyActor))))

(event Collision|EventHit
  (params (MyComp :type Primitive%20Component%20Object%20Reference) (Other :type Actor%20Object%20Reference) (OtherComp :type Primitive%20Component%20Object%20Reference) (bSelfMoved :type Boolean) (HitLocation :type Vector :default "0, 0, 0") (HitNormal :type Vector :default "0, 0, 0") (NormalImpulse :type Vector :default "0, 0, 0") (Hit :type Hit%20Result%20Structure%20%28by%20ref%29))
  (Game|Damage|ApplyRadialDamage (Variables|Default|GetDamage) HitLocation 2e+01 0 0 (Components|GetOwner) 0 true "ECC_Visibility")
  (Effects|SpawnEmitteratLocation "/Game/StarterContent/Particles/P_Explosion.P_Explosion" HitLocation "0, 0, 0" "0.100000,0.100000,0.100000")
  (Actor|DestroyActor))

(fn ConstructionScript)