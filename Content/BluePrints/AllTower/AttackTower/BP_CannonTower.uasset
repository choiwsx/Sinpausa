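; Cannon attack tower that spawns and configures its BP_Cannon weapon actor when play begins.
; After the parent BeginPlay, it reads a fixed row of BP_HRDataTable and spawns the cannon at an offset above itself.
; The cannon receives the row name, the row's attack delay and the tower itself through a pin named ArrowTower.
; The tower's own sphere overlap events are empty.
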(event OnComponentBeginOverlap(Sphere)
  (params (OverlappedComponent :type Primitive%20Component%20Object%20Reference) (OtherActor :type Actor%20Object%20Reference) (OtherComp :type Primitive%20Component%20Object%20Reference) (OtherBodyIndex :type Integer) (bFromSweep :type Boolean) (SweepResult :type Hit%20Result%20Structure%20%28by%20ref%29)))

(event OnComponentEndOverlap(Sphere)
  (params (OverlappedComponent :type Primitive%20Component%20Object%20Reference) (OtherActor :type Actor%20Object%20Reference) (OtherComp :type Primitive%20Component%20Object%20Reference) (OtherBodyIndex :type Integer)))

(event EventBeginPlay
  (|CallParentFunction)
  (bind _returnvalue (Utilities|GetDataTableRow "/Game/HR/BP_HRDataTable.BP_HRDataTable" "1")
    (:then
      (Game|SpawnActorfromClass "/Game/BluePrints/AllTower/AttackTower/BP_Cannon.BP_Cannon_C" (Math|Transform|MakeTransform (+ (Transformation|GetActorLocation) "0.350000, 0,13.000000")) "Undefined" 0 "1" self (.TowerAttackDelay (Utilities|Struct|BreakBP_HRStruct _returnvalue)) 0))))

(event Collision|EventActorBeginOverlap
  (params (OtherActor :type Actor%20Object%20Reference))
  (|CallParentFunction OtherActor) ; 지금 이 노드는 비활성 상태입니다. \n핀을 끌어서 다른 노드를 연결하면 활성화됩니다.
)

(event EventTick
  (params (DeltaSeconds :type Float%20%28single-precision%29))
  (|CallParentFunction DeltaSeconds) ; 지금 이 노드는 비활성 상태입니다. \n핀을 끌어서 다른 노드를 연결하면 활성화됩니다.
)

(fn ConstructionScript
  (|CallParentFunction))