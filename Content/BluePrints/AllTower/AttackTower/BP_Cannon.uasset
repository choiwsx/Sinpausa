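; Cannon attack unit that fires at nearby monsters and destroys itself when its linked ArrowTower is no longer valid.
; Sphere overlap adds monsters to an Enemy list, which is never pruned, and starts a one-second looping timer.
; Each tick of that timer picks the closest valid monster within a fixed XY range, yaws toward it, and spawns a muzzle effect and BP_Projectile, with damage read from BP_HRDataTable.
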(event OnComponentBeginOverlap(Sphere)
  (params (OverlappedComponent :type Primitive%20Component%20Object%20Reference) (OtherActor :type Actor%20Object%20Reference) (OtherComp :type Primitive%20Component%20Object%20Reference) (OtherBodyIndex :type Integer) (bFromSweep :type Boolean) (SweepResult :type Hit%20Result%20Structure%20%28by%20ref%29))
  (bind _asbp_monster_basic (Utilities|Casting|CastToBP_Monster_BASIC OtherActor)) ; 회전을 하면됨
  (Utilities|Array|AddUnique (Variables|Default|GetEnemy) _asbp_monster_basic)
  (if (not (Utilities|Time|IsTimerActivebyHandle (Variables|Default|GetTimeEvent_Attack)))
    (CallFunction|CheckandAttack)))

(event Custom|ProjectileSpawn
  (bind _cannon (Variables|Default|GetCannon))
  ;[1 1 1] 대포 발사
  (Effects|SpawnEmitteratLocation "/Game/GabrielAguiarProd/ToonProjectilesVol1/Particles/Muzzles/P_Muzzle_Bullet01Lowpoly.P_Muzzle_Bullet01Lowpoly" (Transformation|GetSocketLocation _cannon "hand_lBowSocket") (Transformation|GetActorRotation) "0.050000,0.050000,0.050000")
  (bind _returnvalue (Utilities|GetDataTableRow "/Game/HR/BP_HRDataTable.BP_HRDataTable" (Variables|Default|GetStructRow))
    (:then
      (Game|SpawnActorfromClass "/Game/BluePrints/AllTower/AttackTower/BP_Projectile.BP_Projectile_C" (Math|Transform|MakeTransform (Transformation|GetSocketLocation _cannon "hand_lBowSocket") (Transformation|GetActorRotation) "1,1,1") "AlwaysSpawn" self (.TowerDamage (Utilities|Struct|BreakBP_HRStruct _returnvalue)) 0)
      (Utilities|FlowControl|Delay 0.5))))

(event Custom|CheckAndAttack
  (bind _returnvalue (Utilities|Time|SetTimerbyEvent (delegate Custom|CheckAndAttack_Timer) 1.0 true))
  (Variables|Default|SetTimeEvent_Attack _returnvalue))

(event Custom|CheckAndAttack_Timer
  (Variables|Default|SetDistanceToMonster 5e+01)
  (Variables|Default|SetTargetMonster 0)
  (for _array_element (Variables|Default|GetEnemy)
    (Utilities|IsValid _array_element
      (:Is%20Valid
        (if (< (Math|Vector|VectorLengthXY (- (Transformation|GetActorLocation _array_element) (Transformation|GetActorLocation))) (Variables|Default|GetDistanceToMonster))
          (Variables|Default|SetDistanceToMonster (Math|Vector|VectorLengthXY (- (Transformation|GetActorLocation _array_element) (Transformation|GetActorLocation))))
          (Variables|Default|SetTargetMonster _array_element)))))
  (Utilities|IsValid (Variables|Default|GetTargetMonster)
    (:Is%20Valid
      (CallFunction|Rotate (Variables|Default|GetTargetMonster))
      (CallFunction|ProjectileSpawn)
      (if (== (Utilities|Array|Length (Variables|Default|GetEnemy)) 0)
        (Utilities|Time|ClearandInvalidateTimerbyHandle (Variables|Default|GetTimeEvent_Attack))))))

(event Custom|Rotate
  (params (NewParam :type BP%20Monster%20BASIC%20Object%20Reference))
  ;[1 1 1] 회전함수
  (Utilities|IsValid NewParam
    (:Is%20Valid
      (Transformation|SetActorRotation (Math|Rotator|MakeRotator 0.0 0.0 (.yaw (Math|Rotator|FindLookatRotation (Transformation|GetActorLocation) (Transformation|GetActorLocation NewParam))))))))

(event EventTick
  (params (DeltaSeconds :type Float%20%28single-precision%29))
  ;[1 1 1] 타워가 사라지면 공격유닛도 삭제
  (Utilities|IsValid (Variables|Default|GetArrowTower)
    (:Is%20Not%20Valid
      (Actor|DestroyActor))))

(fn ConstructionScript)

(fn CheckTargetCalculation
  (params (In :type Array%20of%20Hit%20Result%20Structures)))

(fn CheckNewTarget)