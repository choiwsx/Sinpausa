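; BP_TeleportLocation is a map actor that, judging by its name, marks a teleport destination with a toggleable particle effect.
; BeginPlay hides the particle system and disables its collision.
; ShowParticle and HideParticle events switch its visibility only when the state differs, without propagating to children.
; It contains no teleport logic and nothing in it calls those two events.
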(event Custom|ShowParticle
  (if (not (Rendering|IsVisible (Variables|Default|GetParticleSystem)))
    (Rendering|SetVisibility (Variables|Default|GetParticleSystem) true false)))

(event Custom|HideParticle
  (if (Rendering|IsVisible (Variables|Default|GetParticleSystem))
    (Rendering|SetVisibility (Variables|Default|GetParticleSystem) false false)))

(event EventBeginPlay
  (Rendering|SetVisibility (Variables|Default|GetParticleSystem) false false)
  (Collision|SetCollisionEnabled (Variables|Default|GetParticleSystem) "NoCollision"))

(event Collision|EventActorBeginOverlap
  (params (OtherActor :type Actor%20Object%20Reference)))

(event EventTick
  (params (DeltaSeconds :type Float%20%28single-precision%29)))

(fn ConstructionScript)