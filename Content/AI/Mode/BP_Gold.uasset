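; BP_Gold is a gold pickup that pops upward with a physics impulse on spawn and spins around its yaw axis.
; When a BP_MotionController overlaps it, it adds its Gold value to the GM_HeroMonster game mode.
; It then plays the amount animation on its Widget_MonsterGold widget, spawns a small gain particle effect and destroys itself after a short delay.
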(event EventBeginPlay
  (Physics|AddImpulse (Variables|Default|GetSphere) (* (Transformation|GetActorUpVector) 1.5e+02) "None" false))

(event Collision|EventActorBeginOverlap
  (params (OtherActor :type Actor%20Object%20Reference))
  (Utilities|Casting|CastToBP_MotionController OtherActor)
  (bind _asgm_hero_monster (Utilities|Casting|CastToGM_HeroMonster (Game|GetGameMode)))
  (Default|AddGold _asgm_hero_monster (Variables|Default|GetGold))
  (bind _aswidget_monster_gold (Utilities|Casting|CastToWidget_MonsterGold (UserInterface|GetUserWidgetObject (Variables|Default|GetWidget))))
  (Default|PlayAnim _aswidget_monster_gold (Variables|Default|GetGold))
  (Utilities|FlowControl|Sequence
    (:then_0
      (Effects|SpawnEmitteratLocation "/Game/GabrielAguiarProd/ToonProjectilesVol1/Particles/Muzzles/P_GainGold.P_GainGold" (Transformation|GetActorLocation) "0, 0, 0" "0.100000,0.100000,0.100000"))
    (:then_1
      (Utilities|FlowControl|Delay 0.5)
      (Actor|DestroyActor))))

(event EventTick
  (params (DeltaSeconds :type Float%20%28single-precision%29))
  (Transformation|AddActorLocalRotation (Math|Rotator|MakeRotator 0.0 0.0 (* DeltaSeconds (Variables|Default|GetRotationSpeed))) false false))

(fn ConstructionScript)