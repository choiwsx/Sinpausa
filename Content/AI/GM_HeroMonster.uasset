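; Game mode for a hero-versus-monster stage, managing gold, life, waves and stage progression.
; BeginPlay reads stage settings from DataTables by GameInstance stage, caches teleport locations and starts a looping timer that spawns the current wave's monsters on a spline.
; CheckMonsterCount starts the next wave once no monsters remain, or fades to the next map or StartMenu after the last.
; Grave_Recovery replaces a grave with a bow hero configured from the tower's level row.
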(event Custom|CheckMonsterCount
  (bind _returnvalue (Game|GetGameInstance))
  (bind _outactors (Actor|GetAllActorsOfClass "/Game/AI/Monster/BP_Monster_BASIC.BP_Monster_BASIC_C"))
  (if (== (Utilities|Array|Length _outactors) 0)
    (Variables|Default|SetWave (Math|Integer|Clamp(Integer) (+ (Variables|Default|GetWave) 1) 0 (Variables|Default|GetTotalWave)))
    (if (< (Variables|Default|GetWave) (Variables|Default|GetTotalWave))
      (CallFunction|NextWave)
      (else
        (bind _outactors_2 (Actor|GetAllActorsOfClass "/Script/Engine.TargetPoint"))
        (Game|SpawnActorfromClass "/Game/AI/Mode/BP_StageParticle.BP_StageParticle_C" (Math|Transform|MakeTransform (Transformation|GetActorLocation (Utilities|Array|Get(acopy) _outactors_2)) "90.000000, 0, 0" "1,1,1") "Undefined" 0 0)
        (Development|PrintString "Next Stage!!!!!!!!!!!!!!!!!!!!!!" true true "(R=0.000000,G=0.660000,B=1.000000,A=1.000000)" 5e+01)
        (CameraFades|StartCameraFade (Game|GetPlayerCameraManager 0) 0.0 1.0 2.0 (Variables|Default|GetNextStageFade) false false)
        (Utilities|FlowControl|Delay 2.0)
        (bind _ashero_monster_game_instance (Utilities|Casting|CastToHeroMonster_GameInstance _returnvalue))
        (if (<= (Variables|/Game/AI/HeroMonster_GameInstance.HeroMonster_GameInstance_C|GetStage _ashero_monster_game_instance) 0)
          (bind _ashero_monster_game_instance_2 (Utilities|Casting|CastToHeroMonster_GameInstance _returnvalue))
          (Variables|/Game/AI/HeroMonster_GameInstance.HeroMonster_GameInstance_C|SetStage _ashero_monster_game_instance_2 (+ (Variables|/Game/AI/HeroMonster_GameInstance.HeroMonster_GameInstance_C|GetStage _ashero_monster_game_instance_2) 1))
          (bind _returnvalue_2 (Utilities|GetDataTableRow "/Game/AI/Monster/DT_StageMonster.DT_StageMonster" (Utilities|String|StringToName (Utilities|String|ToString(Integer) (Variables|/Game/AI/HeroMonster_GameInstance.HeroMonster_GameInstance_C|GetStage _ashero_monster_game_instance_2))))
            (:then
              (Game|OpenLevel(byName) (.MapName (Utilities|Struct|BreakST_Stage _returnvalue_2)))))
          (else
            (Development|PrintString "모든 스테이지 클리어!!!")
            (Utilities|FlowControl|Delay 2.0)
            (Game|OpenLevel(byName) "StartMenu")))))
    (else
      (Development|PrintString (Utilities|String|ToString(Integer) (Utilities|Array|Length _outactors))))))

(event Custom|SpawnMonster
  (bind _ashero_monster_game_instance (Utilities|Casting|CastToHeroMonster_GameInstance (Game|GetGameInstance)))
  (bind _returnvalue (Utilities|GetDataTableRow "/Game/AI/Monster/DT_StageMonster.DT_StageMonster" (Utilities|String|StringToName (Utilities|String|ToString(Integer) (Variables|/Game/AI/HeroMonster_GameInstance.HeroMonster_GameInstance_C|GetStage _ashero_monster_game_instance))))
    (:then
      (for _array_element (.Wave_Monster (Utilities|Struct|BreakST_Stage _returnvalue))
        (if (== (.Wave (Utilities|Struct|BreakST_DATA _array_element)) (Variables|Default|GetWave))
          (bind _returnvalue_2 (Game|SpawnActorfromClass (.Monster (Utilities|Struct|BreakST_DATA _array_element)) (Transformation|GetActorTransform (Utilities|Array|Get(acopy) (stale Custom|NextWave _outactors_2))) "AdjustIfPossibleButAlwaysSpawn" 0 0))
          (Development|PrintString (Utilities|GetClassDisplayName (.Monster (Utilities|Struct|BreakST_DATA _array_element))))
          (bind _asbp_monster_basic (Utilities|Casting|CastToBP_Monster_BASIC _returnvalue_2))
          (Variables|/Game/AI/Monster/BP_Monster_BASIC.BP_Monster_BASIC_C|SetSpline_Ref _asbp_monster_basic (Utilities|Array|Get(acopy) (stale Custom|NextWave _outactors_2)))
          (Math|Integer|IncrementInt (Variables|Default|GetMonsterCount)
            (:%20%20
              (if (not (< (Variables|Default|GetMonsterCount) (.MonsterCount (Utilities|Struct|BreakST_DATA _array_element))))
                (Utilities|Time|ClearandInvalidateTimerbyHandle (Variables|Default|GetSpawnEvent))))))))))

(event Custom|AddGold
  (params (Gold :type Integer))
  (Variables|Default|SetGold (+ Gold (Variables|Default|GetGold))))

(event Custom|NextWave
  (Variables|Default|SetMonsterCount 0)
  (Utilities|FlowControl|Sequence
    (:then_0
      (bind _outactors (Actor|GetAllActorsOfClass "/Game/AI/Hero/BP_HERO_BASE.BP_HERO_BASE_C"))
      (for _array_element _outactors
        (Utilities|Array|Clear (Variables|/Game/AI/Hero/BP_HERO_BASE.BP_HERO_BASE_C|GetBattleMonsterArray _array_element))))
    (:then_1
      (bind _outactors_2 (Actor|GetAllActorsOfClass "/Game/AI/Monster/Spline_Base.Spline_Base_C"))
      (bind _returnvalue (Utilities|Time|SetTimerbyEvent (delegate Custom|SpawnMonster) 1.0 true))
      (Variables|Default|SetSpawnEvent _returnvalue))))

(event Custom|Grave_Recovery
  (params (Location :type Vector) (Grave :type BP%20Grave%20Object%20Reference))
  (bind _outactors (Actor|GetAllActorsOfClass "/Game/BluePrints/AllTower/BarracksTower/BP_BowHeroTower.BP_BowHeroTower_C"))
  (Utilities|IsValid (Utilities|Array|Get(acopy) _outactors)
    (:Is%20Valid
      (bind _returnvalue (Utilities|GetDataTableRow "/Game/AI/Hero/Struct/DT_BowHero.DT_BowHero" (Utilities|String|StringToName (Utilities|String|ToString(Integer) (Variables|/Game/BluePrints/AllTower/BarracksTower/BP_BowHeroTower.BP_BowHeroTower_C|Getlevel (Utilities|Array|Get(acopy) _outactors)))))
        (:then
          (bind _returnvalue_2 (Game|SpawnActorfromClass "/Game/AI/Hero/BP_BasicBow.BP_BasicBow_C" (Math|Transform|MakeTransform Location (.rotation (Transformation|GetActorTransform (Utilities|Array|Get(acopy) _outactors))) "1,1,1") "AlwaysSpawn" 0 0 0))
          (Variables|/Game/AI/Hero/BP_HERO_BASE.BP_HERO_BASE_C|SetMaxHP _returnvalue_2 (.MaxHP (Utilities|Struct|BreakST_Hero _returnvalue)))
          (Variables|/Game/AI/Hero/BP_HERO_BASE.BP_HERO_BASE_C|SetBasicDamage _returnvalue_2 (.BasicDamage (Utilities|Struct|BreakST_Hero _returnvalue)))
          (Variables|/Game/AI/Hero/BP_HERO_BASE.BP_HERO_BASE_C|SetInt_BasicAttackMontageCount _returnvalue_2 (.AttackMontageCount (Utilities|Struct|BreakST_Hero _returnvalue)))
          (Class|SkinnedMeshComponent|SetSkeletalMesh (Variables|/Game/AI/Hero/BP_BasicSword.BP_BasicSword_C|GetBelt _returnvalue_2) (.Belt (Utilities|Struct|BreakST_Hero _returnvalue)) true)
          (Class|SkinnedMeshComponent|SetSkeletalMesh (Variables|/Game/AI/Hero/BP_BasicSword.BP_BasicSword_C|GetShoe _returnvalue_2) (.Shoe (Utilities|Struct|BreakST_Hero _returnvalue)) true)
          (Class|SkinnedMeshComponent|SetSkeletalMesh (Variables|/Game/AI/Hero/BP_BasicSword.BP_BasicSword_C|GetGlove _returnvalue_2) (.Glove (Utilities|Struct|BreakST_Hero _returnvalue)) true)
          (Class|SkinnedMeshComponent|SetSkeletalMesh (Variables|/Game/AI/Hero/BP_BasicSword.BP_BasicSword_C|GetHeadGears _returnvalue_2) (.HeadGears (Utilities|Struct|BreakST_Hero _returnvalue)) true)
          (Class|SkinnedMeshComponent|SetSkeletalMesh (Variables|/Game/AI/Hero/BP_BasicSword.BP_BasicSword_C|GetHair _returnvalue_2) (.Hair (Utilities|Struct|BreakST_Hero _returnvalue)) true)
          (Actor|DestroyActor Grave))))))

(event EventBeginPlay
  (Utilities|FlowControl|Sequence
    (:then_0
      (bind _outactors (Actor|GetAllActorsOfClass "/Game/AI/Monster/Spline_Base.Spline_Base_C"))
      (bind _returnvalue (Utilities|Time|SetTimerbyEvent (delegate Custom|SpawnMonster) 1.0 true))
      (Variables|Default|SetSpawnEvent _returnvalue))
    (:then_1
      (bind _ashero_monster_game_instance (Utilities|Casting|CastToHeroMonster_GameInstance (Game|GetGameInstance)))
      (bind _returnvalue_2 (Utilities|GetDataTableRow "/Game/AI/Mode/DT_StageGold.DT_StageGold" (Utilities|String|StringToName (Utilities|String|ToString(Integer) (Variables|/Game/AI/HeroMonster_GameInstance.HeroMonster_GameInstance_C|GetStage _ashero_monster_game_instance))))
        (:then
          (Variables|Default|SetGold (.Gold (Utilities|Struct|BreakST_StageGold _returnvalue_2)))
          (Variables|Default|SetLife (.Life (Utilities|Struct|BreakST_StageGold _returnvalue_2))))))
    (:then_2
      (bind _ashero_monster_game_instance_2 (Utilities|Casting|CastToHeroMonster_GameInstance (Game|GetGameInstance)))
      (bind _returnvalue_3 (Utilities|GetDataTableRow "/Game/AI/Monster/DT_StageMonster.DT_StageMonster" (Utilities|String|StringToName (Utilities|String|ToString(Integer) (Variables|/Game/AI/HeroMonster_GameInstance.HeroMonster_GameInstance_C|GetStage _ashero_monster_game_instance_2))))
        (:then
          (Variables|Default|SetTotalWave (Utilities|Array|Length (.Wave_Monster (Utilities|Struct|BreakST_Stage _returnvalue_3)))))))
    (:then_3
      (bind _outactors_2 (Actor|GetAllActorsOfClass "/Game/Maps/BP_TeleportLocation.BP_TeleportLocation_C"))
      (Variables|Default|SetTeleportArray _outactors_2))))

(event EventTick
  (params (DeltaSeconds :type Float%20%28single-precision%29)))

(fn ConstructionScript)