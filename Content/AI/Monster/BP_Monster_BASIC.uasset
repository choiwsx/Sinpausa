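; Base monster with stats from DT_Monster that follows a spline while in PEACE and fights heroes.
; SetState mirrors state to the AI blackboard and sets speed and montages; pawn sensing targets the nearest hero within range to chase.
; AnyDamage updates the HP widget, flashes the outline and starts fire, ice or thunder timer effects.
; Death plays a montage with material fade, drops gold and notifies the game mode; AggroCheck is an empty hook.
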(event OnSeePawn(PawnSensing)
  (params (Pawn :type Pawn%20Object%20Reference))
  ;[1 1 1] OnSeePawn 이벤트
  (bind _asbp_hero_base (Utilities|Casting|CastToBP_HERO_BASE Pawn))
  (if (Utilities|Enum|NotEqual(Enum) (Variables|/Game/AI/Hero/BP_HERO_BASE.BP_HERO_BASE_C|GetCurrentStatePawn _asbp_hero_base) "NewEnumerator3")
    (Variables|Default|SetDistanceToHero 5e+01)
    (Variables|Default|SetTargetHero 0)
    (bind _outactors (Actor|GetAllActorsOfClass "/Game/AI/Hero/BP_HERO_BASE.BP_HERO_BASE_C"))
    (for _array_element _outactors
      (if (< (Math|Vector|VectorLength (- (Transformation|GetActorLocation) (Transformation|GetActorLocation _array_element))) (Variables|Default|GetDistanceToHero))
        (Variables|Default|SetDistanceToHero (Math|Vector|VectorLength (- (Transformation|GetActorLocation) (Transformation|GetActorLocation _array_element))))
        (Variables|Default|SetTargetHero _array_element)))
    (Utilities|IsValid (Variables|Default|GetTargetHero)
      (:Is%20Valid
        (if (Utilities|Enum|NotEqual(Enum) (Variables|/Game/AI/Hero/BP_HERO_BASE.BP_HERO_BASE_C|GetCurrentStatePawn _array_element) "NewEnumerator3")
          (Variables|Actor|SetInstigator (Variables|Default|GetTargetHero))
          (CallFunction|SetState "NewEnumerator1")
          (Utilities|Array|AddUnique (Variables|/Game/AI/Hero/BP_HERO_BASE.BP_HERO_BASE_C|GetMonsters (Variables|Default|GetTargetHero)) self)
          (Utilities|FlowControl|DoOnce false
            (:Completed
              (AI|Components|Blackboard|SetValueasVector (AI|GetBlackboard (AI|GetAIController self)) (Variables|Default|GetTarget) (Transformation|GetActorLocation))
              (Development|PrintString "sen")))
          (else
            (Variables|Default|SetDistanceToHero 9999.0 :!label _label)
            (Variables|Default|SetTargetHero 0))))
      (:Is%20Not%20Valid
        (goto _label)))))

(event Custom|SetState
  (params (NewState :type BPE_MonsterState%20Enum :default "NewEnumerator0"))
  (bind _returnvalue (Pawn|GetController))
  (bind _returnvalue_2 (AI|GetBlackboard _returnvalue))
  ;[1 1 1] SetState 이벤트
  (Development|PrintString (Utilities|String|EnumtoString NewState))
  (if (Utilities|Enum|NotEqual(Enum) (Variables|Default|GetCurrentState) "NewEnumerator3")
    (bind _output_get (Variables|Default|SetCurrentState NewState))
    (Utilities|FlowControl|Sequence
      (:then_0
        (Utilities|IsValid _returnvalue_2
          (:Is%20Valid
            (AI|Components|Blackboard|SetValueasEnum _returnvalue_2 (Variables|Default|GetStateKey) _output_get))))
      (:then_1
        (switch Utilities|FlowControl|Switch|SwitchonBPE_MonsterState (Variables|Default|GetCurrentState)
          (:NewEnumerator0
            (bind _output_get_2 (Variables|/Script/Engine.CharacterMovementComponent|SetMaxWalkSpeed (Variables|Character|GetCharacterMovement) 5.0))
            (Variables|Default|SetCurrentSpeed _output_get_2))
          (:NewEnumerator1
            (bind _output_get_3 (Variables|/Script/Engine.CharacterMovementComponent|SetMaxWalkSpeed (Variables|Character|GetCharacterMovement) 2e+01))
            (Variables|Default|SetCurrentSpeed _output_get_3))
          (:NewEnumerator2
            (bind _output_get_4 (Variables|/Script/Engine.CharacterMovementComponent|SetMaxWalkSpeed (Variables|Character|GetCharacterMovement) 0.0))
            (Variables|Default|SetCurrentSpeed _output_get_4)
            (Utilities|IsValid (Variables|Default|GetAttack_Montage)
              (:Is%20Valid
                (Animation|Montage|PlayMontage (Variables|Default|GetSkeletalMesh) (Variables|Default|GetAttack_Montage) 1.0 0.0 (Utilities|String|StringToName (Utilities|String|ToString(Text) (Utilities|Text|FormatText "Attack{Num}" (Math|Random|RandomIntegerinRange 1 (Variables|Default|GetInt_MaxAttackMontage)))))
                  (:OnCompleted
                    (CallFunction|AggroCheck))))))
          (:NewEnumerator3
            (bind _output_get_5 (Variables|/Script/Engine.CharacterMovementComponent|SetMaxWalkSpeed (Variables|Character|GetCharacterMovement) 0.0))
            (Variables|Default|SetCurrentSpeed _output_get_5)
            (Animation|StopAnimMontage 0))
          (:NewEnumerator5
            (bind _output_get_6 (Variables|/Script/Engine.CharacterMovementComponent|SetMaxWalkSpeed (Variables|Character|GetCharacterMovement) 0.0))
            (Variables|Default|SetCurrentSpeed _output_get_6))
          (:NewEnumerator6
            (Variables|/Script/Engine.CharacterMovementComponent|SetMaxWalkSpeed (Variables|Character|GetCharacterMovement) 2e+01)))))))

(event Custom|Combo2_monster
  (CallFunction|SetState "NewEnumerator5"))

(event Custom|AggroCheck)

(event Custom|BasicAttack
  (params (Damage :type Float%20%28single-precision%29))
  (bind _returnvalue (Transformation|GetActorLocation))
  ;[1 1 1] 몬스터 베이직 어택
  (bind _outactors (Actor|GetAllActorsOfClass "BP_Monster_BASIC_C"))
  (bind _outhit (Class|KismetSystemLibrary|CapsuleTraceSingleforObjects _returnvalue (+ _returnvalue (* (Transformation|GetActorForwardVector) 6.0)) 4.0 3.0 (Utilities|Array|MakeArray "ObjectTypeQuery3") false _outactors "None" true "(R=0.000000,G=0.207014,B=1.000000,A=1.000000)" "(R=1.000000,G=0.000000,B=0.951921,A=1.000000)"))
  (bind _asbp_hero_base (Utilities|Casting|CastToBP_HERO_BASE (.HitActor (Collision|BreakHitResult _outhit))))
  (Utilities|IsValid _asbp_hero_base
    (:Is%20Valid
      (Physics|AddImpulse (Variables|/Script/Engine.Character|GetCharacterMovement _asbp_hero_base) (* (Transformation|GetActorForwardVector _asbp_hero_base) -2e+01) false)
      (Effects|SpawnEmitteratLocation "/Game/SimpleCartoonFX/FX/Hit.Hit" (Transformation|GetActorLocation _asbp_hero_base) "0, 0, 0" "0.050000,0.050000,0.050000")
      (Game|Damage|ApplyDamage _asbp_hero_base Damage 0 self))))

(event Custom|Combo2_Impulse
  (Physics|AddImpulse (Variables|Character|GetCharacterMovement) (* (Transformation|GetActorForwardVector) -5.0) true))

(event Custom|Counter
  (params (Hero :type BP%20HERO%20BASE%20Object%20Reference))
  (if (Utilities|Enum|NotEqual(Enum) (Variables|/Game/AI/Hero/BP_HERO_BASE.BP_HERO_BASE_C|GetCurrentStatePawn Hero) "NewEnumerator3")
    (CallFunction|AggroCheck)))

(event Custom|DOT
  (bind _die_montage (Variables|Default|GetDie_Montage))
  ;[1 1 1] 불 데미지
  (Utilities|IsValid (stale Game|Damage|EventAnyDamage _asbp_fire_type)
    (:Is%20Valid
      (Variables|Default|SetCurrentHP (- (Variables|Default|GetCurrentHP) (Variables|/Game/BluePrints/AllTower/MagicTower/DamageType/BP_DamageBase.BP_DamageBase_C|GetDOT (stale Game|Damage|EventAnyDamage _asbp_fire_type))))
      (bind _result (Math|Integer|IncrementInt (Variables|Default|GetCount))
        (:%20%20
          (if (> _result (Variables|/Game/BluePrints/AllTower/MagicTower/DamageType/BP_DamageBase.BP_DamageBase_C|GetDuration (stale Game|Damage|EventAnyDamage _asbp_fire_type))) ; 시간이 다 되면 True
            (Utilities|Time|PauseTimerbyHandle (Variables|Default|GetTiemHandle))
            ;[1 1 1] AnyDamage 이벤트
            (Progress|SetPercent (Variables|/Game/AI/Monster/Widget/Widget_MonsterHP.Widget_MonsterHP_C|GetHP (stale Game|Damage|EventAnyDamage _aswidget_monster_hp)) (/ (Variables|Default|GetCurrentHP) (Variables|Default|GetMaxHP)) :!label _label)
            (if (<= (Variables|Default|GetCurrentHP) 0.0)
              (CallFunction|SetState "NewEnumerator3")
              (Collision|SetCollisionEnabled (Variables|Collision|GetCapsuleComponent) "PhysicsOnly")
              (Utilities|FlowControl|Sequence
                (:then_0
                  (bind _asbp_hero_base (Utilities|Casting|CastToBP_HERO_BASE (stale Game|Damage|EventAnyDamage DamageCauser)))
                  (Default|AggroCheck _asbp_hero_base)
                  (Default|RemoveBattleMonster _asbp_hero_base self))
                (:then_1
                  (Utilities|IsValid _die_montage
                    (:Is%20Valid
                      (Animation|Montage|PlayMontage (Variables|Default|GetSkeletalMesh) _die_montage 1.5 0.0 (Utilities|String|StringToName (Utilities|String|ToString(Text) (Utilities|Text|FormatText "Death{number}" (Math|Random|RandomIntegerinRange 1 (Variables|Default|GetInt_MaxDieMontage)))))
                        (:then
                          (bind _power (Timeline|타임라인_4 PlayFromStart)
                            (:Update
                              (Rendering|Material|SetScalarParameterValueonMaterials (Variables|Default|GetSkeletalMesh) "Amount" _power))))
                        (:OnCompleted
                          (Utilities|FlowControl|Sequence
                            (:then_0
                              (Game|SpawnActorfromClass "/Game/AI/Mode/BP_Gold.BP_Gold_C" (Math|Transform|MakeTransform (Transformation|GetActorLocation) "0, 0, 0" "1,1,1") "Undefined" 0 (Variables|Default|GetGold) 0)
                              (Actor|DestroyActor))
                            (:then_1
                              (bind _asgm_hero_monster (Utilities|Casting|CastToGM_HeroMonster (Game|GetGameMode)))
                              (Default|CheckMonsterCount _asgm_hero_monster))))))))))
            (else
              (Progress|SetPercent (Variables|/Game/AI/Monster/Widget/Widget_MonsterHP.Widget_MonsterHP_C|GetHP (stale Game|Damage|EventAnyDamage _aswidget_monster_hp)) (/ (Variables|Default|GetCurrentHP) (Variables|Default|GetMaxHP))) ; 데미지 받을떄 마다 죽음 측정
              (if (<= (Variables|Default|GetCurrentHP) 0.0) ; 죽으면 DOT정지+죽음판정
                (Utilities|Time|PauseTimerbyHandle (Variables|Default|GetTiemHandle))
                (goto _label)))))))))

(event Custom|Shock
  ;[1 1 1] 번개 데미지
  (bind _result (Math|Integer|IncrementInt (Variables|Default|GetCount))
    (:%20%20
      (if (> _result (Variables|/Game/BluePrints/AllTower/MagicTower/DamageType/BP_DamageBase.BP_DamageBase_C|GetDuration (stale Game|Damage|EventAnyDamage _asbp_thunder_type))) ; 시간이 다 되면 True
        (Utilities|Time|PauseTimerbyHandle (Variables|Default|GetTiemHandle))
        (Variables|Default|SetCurrentSpeed 5.0)
        (Variables|Default|SetCount 0)))))

(event Custom|Slow
  ;[1 1 1] 얼음 데미지
  (bind _result (Math|Integer|IncrementInt (Variables|Default|GetCount))
    (:%20%20
      (if (> _result (Variables|/Game/BluePrints/AllTower/MagicTower/DamageType/BP_DamageBase.BP_DamageBase_C|GetDuration (stale Game|Damage|EventAnyDamage _asbp_ice_type))) ; 시간이 다 되면 True
        (Utilities|Time|PauseTimerbyHandle (Variables|Default|GetTiemHandle))
        (Variables|Default|SetCurrentSpeed 5.0)
        (Variables|Default|SetCount 0)))))

(event EventBeginPlay
  ;[1 1 1] Begin Play 이벤트
  (CallFunction|SetState "NewEnumerator0")
  (Variables|Default|SetOffset (Math|Random|RandomFloatinRange -7.0 7.0))
  (bind _returnvalue (Utilities|GetDataTableRow "/Game/AI/Monster/Struct/DT_Monster.DT_Monster" (Utilities|String|StringToName (Utilities|String|ToString(Integer) (Variables|Default|GetLevel))))
    (:then
      (Variables|Default|SetMaxHP (.MaxHP (Utilities|Struct|BreakST_Monster _returnvalue)))
      (Variables|Default|SetDamage (.BasicDamage (Utilities|Struct|BreakST_Monster _returnvalue)))
      (Variables|Default|SetGold (.Gold (Utilities|Struct|BreakST_Monster _returnvalue)))
      (Variables|Default|SetCurrentSpeed (.Start_MoveSpeed (Utilities|Struct|BreakST_Monster _returnvalue)))
      (Variables|Default|SetInt_MaxAttackMontage (.AttackMontageCount (Utilities|Struct|BreakST_Monster _returnvalue)))
      (Variables|Default|SetCurrentHP (Variables|Default|GetMaxHP))
      (bind _aswidget_monster_hp (Utilities|Casting|CastToWidget_MonsterHP (UserInterface|GetUserWidgetObject (Variables|Default|GetWidget))))
      (Progress|SetPercent (Variables|/Game/AI/Monster/Widget/Widget_MonsterHP.Widget_MonsterHP_C|GetHP _aswidget_monster_hp) (/ (Variables|Default|GetCurrentHP) (Variables|Default|GetMaxHP))))))

(event Collision|EventActorBeginOverlap
  (params (OtherActor :type Actor%20Object%20Reference))
  (|CallParentFunction OtherActor) ; 지금 이 노드는 비활성 상태입니다. \n핀을 끌어서 다른 노드를 연결하면 활성화됩니다.
)

(event EventTick
  (params (DeltaSeconds :type Float%20%28single-precision%29))
  (bind _spline_ref (Variables|Default|GetSpline_Ref))
  (bind _spline (Variables|/Game/AI/Monster/Spline_Base.Spline_Base_C|GetSpline _spline_ref))
  ;[1 1 1] Tick 이벤트
  (Utilities|FlowControl|Sequence
    (:then_0
      (if (Utilities|Enum|Equal(Enum) (Variables|Default|GetCurrentState) "NewEnumerator6")
        (if (<= (Math|Vector|VectorLength (- (AI|Components|Blackboard|GetValueasVector (AI|GetBlackboard 0) (Variables|Default|GetTarget)) (Transformation|GetActorLocation))) 3.0)
          (CallFunction|SetState "NewEnumerator0"))))
    (:then_1
      (if (Utilities|Enum|Equal(Enum) (Variables|Default|GetCurrentState) "NewEnumerator0")
        (Utilities|IsValid (Variables|Default|GetSpline_Ref)
          (:Is%20Valid
            (Variables|Default|SetDistanceAlongSpline (+ (* (* (Variables|Default|GetCurrentSpeed) (Variables|Default|GetAxisValue)) (Utilities|Time|GetWorldDeltaSeconds)) (Variables|Default|GetDistanceAlongSpline)))
            (Transformation|SetActorLocation (Math|Vector|MakeVector (+ (Variables|Default|GetOffset) (.x (Spline|GetLocationatDistanceAlongSpline _spline (Variables|Default|GetDistanceAlongSpline) "World"))) (+ (.y (Spline|GetLocationatDistanceAlongSpline _spline (Variables|Default|GetDistanceAlongSpline) "World")) (Variables|Default|GetOffset)) (.z (Transformation|GetActorLocation))) false false)
            (Transformation|SetActorRelativeRotation (Spline|GetRotationatDistanceAlongSpline _spline (Variables|Default|GetDistanceAlongSpline) "World"))
            (Variables|Default|SetB_PEACE_WALK true)))
        (else
          (Variables|Default|SetB_PEACE_WALK false))))))

(event Game|Damage|EventAnyDamage
  (params (Damage :type Float%20%28single-precision%29) (DamageType :type Damage%20Type%20Object%20Reference) (InstigatedBy :type Controller%20Object%20Reference) (DamageCauser :type Actor%20Object%20Reference))
  (bind _die_montage (Variables|Default|GetDie_Montage))
  ;[1 1 1] AnyDamage 이벤트
  (if (Utilities|Enum|NotEqual(Enum) (Variables|Default|GetCurrentState) "NewEnumerator3")
    (Utilities|FlowControl|Sequence
      (:then_1
        (bind _aswidget_monster_hp (Utilities|Casting|CastToWidget_MonsterHP (UserInterface|GetUserWidgetObject (Variables|Default|GetWidget))))
        (Variables|Default|SetCurrentHP (- (Variables|Default|GetCurrentHP) Damage))
        (Progress|SetPercent (Variables|/Game/AI/Monster/Widget/Widget_MonsterHP.Widget_MonsterHP_C|GetHP _aswidget_monster_hp) (/ (Variables|Default|GetCurrentHP) (Variables|Default|GetMaxHP))) ; 데미지 받을떄 마다 죽음 측정
        (if (<= (Variables|Default|GetCurrentHP) 0.0) ; 죽으면 DOT정지+죽음판정
          (Progress|SetPercent (Variables|/Game/AI/Monster/Widget/Widget_MonsterHP.Widget_MonsterHP_C|GetHP _aswidget_monster_hp) (/ (Variables|Default|GetCurrentHP) (Variables|Default|GetMaxHP)) :!label _label)
          (if (<= (Variables|Default|GetCurrentHP) 0.0)
            (CallFunction|SetState "NewEnumerator3")
            (Collision|SetCollisionEnabled (Variables|Collision|GetCapsuleComponent) "PhysicsOnly")
            (Utilities|FlowControl|Sequence
              (:then_0
                (bind _asbp_hero_base (Utilities|Casting|CastToBP_HERO_BASE DamageCauser))
                (Default|AggroCheck _asbp_hero_base)
                (Default|RemoveBattleMonster _asbp_hero_base self))
              (:then_1
                (Utilities|IsValid _die_montage
                  (:Is%20Valid
                    (Animation|Montage|PlayMontage (Variables|Default|GetSkeletalMesh) _die_montage 1.5 0.0 (Utilities|String|StringToName (Utilities|String|ToString(Text) (Utilities|Text|FormatText "Death{number}" (Math|Random|RandomIntegerinRange 1 (Variables|Default|GetInt_MaxDieMontage)))))
                      (:then
                        (bind _power (Timeline|타임라인_4 PlayFromStart)
                          (:Update
                            (Rendering|Material|SetScalarParameterValueonMaterials (Variables|Default|GetSkeletalMesh) "Amount" _power))))
                      (:OnCompleted
                        (Utilities|FlowControl|Sequence
                          (:then_0
                            (Game|SpawnActorfromClass "/Game/AI/Mode/BP_Gold.BP_Gold_C" (Math|Transform|MakeTransform (Transformation|GetActorLocation) "0, 0, 0" "1,1,1") "Undefined" 0 (Variables|Default|GetGold) 0)
                            (Actor|DestroyActor))
                          (:then_1
                            (bind _asgm_hero_monster (Utilities|Casting|CastToGM_HeroMonster (Game|GetGameMode)))
                            (Default|CheckMonsterCount _asgm_hero_monster))))))))))
          (else
            ;[1 1 1] 불 데미지
            (bind _asbp_fire_type (Utilities|Casting|CastToBP_FireType DamageType)
              (:then
                (Utilities|IsValid _asbp_fire_type
                  (:Is%20Valid
                    (bind _returnvalue (Utilities|Time|SetTimerbyEvent (delegate Custom|DOT) 1.0 true))
                    (Variables|Default|SetTiemHandle _returnvalue))))
              (:CastFailed
                ;[1 1 1] 얼음 데미지
                (bind _asbp_ice_type (Utilities|Casting|CastToBP_IceType DamageType)
                  (:then
                    (Variables|Default|SetCurrentSpeed (* (Variables|Default|GetCurrentSpeed) (Variables|/Game/BluePrints/AllTower/MagicTower/DamageType/BP_DamageBase.BP_DamageBase_C|GetFinalSpeed _asbp_ice_type)))
                    (bind _returnvalue_2 (Utilities|Time|SetTimerbyEvent (delegate Custom|Slow) 1.0 true))
                    (Variables|Default|SetTiemHandle _returnvalue_2)
                    (goto _label))
                  (:CastFailed
                    ;[1 1 1] 번개 데미지
                    (bind _asbp_thunder_type (Utilities|Casting|CastToBP_ThunderType DamageType)
                      (:then
                        (Variables|Default|SetCurrentSpeed (* (Variables|Default|GetCurrentSpeed) (Variables|/Game/BluePrints/AllTower/MagicTower/DamageType/BP_DamageBase.BP_DamageBase_C|GetFinalSpeed _asbp_thunder_type)))
                        (bind _returnvalue_3 (Utilities|Time|SetTimerbyEvent (delegate Custom|Shock) 1.0 true))
                        (Variables|Default|SetTiemHandle _returnvalue_3))
                      (:CastFailed
                        (goto _label))))))))))
      (:then_2
        (bind _새_트랙_0 (Timeline|피격타임라인 PlayFromStart)
          (:Update
            (Rendering|Material|SetScalarParameterValueonMaterials (Variables|Default|GetSkeletalMesh) "OutlineEmissive" _새_트랙_0)))))))

(fn ConstructionScript
  (|CallParentFunction))