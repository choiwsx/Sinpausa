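; Monster component that applies secondary damage-over-time after a hit, presumably for fire damage.
; HandleDamage stores the damage type and causer, then starts a looping one-second timer that applies DOT through the owning BP_Monster_BASIC.
; Each tick updates health percentage and checks death, calling OnDead with the causer and clearing references.
; Exceeding Duration only resets the tick counter; the stored timer handle is never cleared.
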(event Custom|ResetReferences
  ;[1 1 1] 참조 변수 초기화
  (Variables|Default|SetRefDamageType 0)
  (Variables|Default|SetRefDamageCauser 0))

(event Custom|FinishTimer
  ;[1 1 1] 타이머 종료
  (Variables|Default|SetCount 0))

(event Custom|AfterMainDamage
  (bind _refmonster (Variables|Default|GetRefMonster))
  (bind _refmonster_2 (Variables|Default|GetRefMonster))
  ;[1 1 1] 2차 데미지 효과 처리
  (Utilities|IsValid (Variables|Default|GetRefDamageType)
    (:Is%20Valid
      (Default|ProcessDamage (Variables|Default|GetRefMonster) (Variables|/Game/BluePrints/AllTower/MagicTower/DamageType/BP_DamageBase.BP_DamageBase_C|GetDOT (Variables|Default|GetRefDamageType)))
      (bind _result (Math|Integer|IncrementInt (Variables|Default|GetCount))
        (:%20%20
          (if (> _result (Variables|/Game/BluePrints/AllTower/MagicTower/DamageType/BP_DamageBase.BP_DamageBase_C|GetDuration (Variables|Default|GetRefDamageType))) ; True 시간초과 False 효과지속
            (CallFunction|FinishTimer)
            (Default|MultiSetPercent (Variables|Default|GetRefMonster) (/ (Variables|/Game/AI/Monster/BP_Monster_BASIC.BP_Monster_BASIC_C|GetCurrentHP _refmonster_2) (Variables|/Game/AI/Monster/BP_Monster_BASIC.BP_Monster_BASIC_C|GetMaxHP _refmonster_2)))
            (bind _isdead (Default|CheckifDead (Variables|Default|GetRefMonster)))
            (if _isdead
              (Default|OnDead (Variables|Default|GetRefMonster) (Variables|Default|GetRefDamageCauser))
              (CallFunction|ResetReferences))
            (else
              (Default|MultiSetPercent (Variables|Default|GetRefMonster) (/ (Variables|/Game/AI/Monster/BP_Monster_BASIC.BP_Monster_BASIC_C|GetCurrentHP _refmonster) (Variables|/Game/AI/Monster/BP_Monster_BASIC.BP_Monster_BASIC_C|GetMaxHP _refmonster)))
              (bind _isdead_2 (Default|CheckifDead (Variables|Default|GetRefMonster)))
              (if _isdead_2 ; Ture효과 지속중 사망 False 효과 지속
                (Default|OnDead (Variables|Default|GetRefMonster) (Variables|Default|GetRefDamageCauser))
                (CallFunction|FinishTimer)
                (CallFunction|ResetReferences)))))))))

(event EventBeginPlay
  (bind _asbp_monster_basic (Utilities|Casting|CastToBP_Monster_BASIC (Components|GetOwner)))
  (Variables|Default|SetRefMonster _asbp_monster_basic)
  (bind _aswidget_monster_hp (Utilities|Casting|CastToWidget_MonsterHP (UserInterface|GetUserWidgetObject (Variables|/Game/AI/Monster/BP_Monster_BASIC.BP_Monster_BASIC_C|GetWidget (Variables|Default|GetRefMonster)))))
  (Variables|Default|SetRefMonsterHP _aswidget_monster_hp))

(event EventHandleDamage
  (params (DamageType :type BP%20Damage%20Base%20Object%20Reference) (DamageCauser :type Actor%20Object%20Reference))
  ;[1 1 1] 2차 데미지 효과 처리
  (bind _output_get (Variables|Default|SetRefDamageType DamageType))
  (Variables|Default|SetRefDamageCauser DamageCauser)
  (Utilities|IsValid _output_get
    (:Is%20Valid
      (bind _returnvalue (Utilities|Time|SetTimerbyEvent (delegate Custom|AfterMainDamage) 1.0 true))
      (Variables|Default|SetTimeHandle _returnvalue))))